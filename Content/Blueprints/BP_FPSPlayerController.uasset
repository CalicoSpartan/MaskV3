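; FPS player controller Blueprint that creates and updates the client's in-game HUD, score bars and team scoreboard.
; Trigger events forward to handlers that create each widget set once, also passing the HUD to BP_GameState.
; The scoreboard builds two team panels with an unpopulated row per controller in the GameState's team arrays.
; Score updates set team and rival percentages, while the player stats update is an empty stub.
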(event Custom|UpdateScore
  (bind _scoreui (Variables|Default|GetScoreUI))
  ;[1 1 1] ScoreUI
  (Utilities|IsValid (Variables|Default|GetScoreUI)
    (:Is%20Valid
      (Progress|SetPercent (Variables|/Game/UI/ScoreUI.ScoreUI_C|GetMyScore _scoreui) (Variables|Default|GetTeamScorePercent))
      (Progress|SetPercent (Variables|/Game/UI/ScoreUI.ScoreUI_C|GetEnemyScore _scoreui) (Variables|Default|GetRivalScorePercent)))))

(event Custom|AddGameUIToClient
  ;[1 1 1] GameUI
  (Utilities|IsValid (Variables|Default|GetInGameUI)
    (:Is%20Not%20Valid
      (bind _returnvalue (UserInterface|CreateWidget "/Game/UI/InGameUI.InGameUI_C"))
      (bind _output_get (Variables|Default|SetInGameUI _returnvalue))
      (bind _asbp_game_state (Utilities|Casting|CastToBP_GameState (Game|GetGameState)))
      (Variables|/Game/Blueprints/BP_GameState.BP_GameState_C|SetUI _asbp_game_state _returnvalue)
      (UserInterface|Viewport|AddtoViewport _output_get 0)
      (bind _returnvalue_2 (UserInterface|CreateWidget "/Game/UI/ScoreUI.ScoreUI_C"))
      (bind _output_get_2 (Variables|Default|SetScoreUI _returnvalue_2))
      (UserInterface|Viewport|AddtoViewport _output_get_2 1))))

(event Custom|UpdatePlayerStats)

(event Custom|AddScoreBoardToClient
  ;[1 1 1] base scoreboard
  (Utilities|IsValid (Variables|Default|GetScoreBoardUI)
    (:Is%20Not%20Valid
      (bind _returnvalue (UserInterface|CreateWidget "/Game/UI/ScoreBoardUI.ScoreBoardUI_C"))
      (Variables|Default|SetScoreBoardUI _returnvalue)
      (bind _returnvalue_2 (UserInterface|CreateWidget "/Game/UI/TeamScoreBoard.TeamScoreBoard_C"))
      (bind _output_get (Variables|Default|SetTeam1Stats _returnvalue_2))
      (Rendering|Components|TextRender|SetText (Variables|/Game/UI/TeamScoreBoard.TeamScoreBoard_C|GetTeamNameHere _output_get) "Team1")
      (Class|VerticalBox|AddChildtoVerticalBox (Variables|/Game/UI/ScoreBoardUI.ScoreBoardUI_C|GetVerticalScoreBox (Variables|Default|GetScoreBoardUI)) _output_get)
      (bind _returnvalue_3 (UserInterface|CreateWidget "/Game/UI/TeamScoreBoard.TeamScoreBoard_C"))
      (bind _output_get_2 (Variables|Default|SetTeam2Stats _returnvalue_3))
      (Rendering|Components|TextRender|SetText (Variables|/Game/UI/TeamScoreBoard.TeamScoreBoard_C|GetTeamNameHere _output_get_2) "Team2")
      (Class|VerticalBox|AddChildtoVerticalBox (Variables|/Game/UI/ScoreBoardUI.ScoreBoardUI_C|GetVerticalScoreBox (Variables|Default|GetScoreBoardUI)) _output_get_2)
      (bind _asbp_game_state (Utilities|Casting|CastToBP_GameState (Game|GetGameState)))
      (for _array_element (Variables|/Script/FPSProject.FPSGameState|GetTeam1PlayerControllers _asbp_game_state)
        (bind _returnvalue_4 (UserInterface|CreateWidget "/Game/UI/PlayerStats.PlayerStats_C"))
        (Class|VerticalBox|AddChildtoVerticalBox (Variables|/Game/UI/TeamScoreBoard.TeamScoreBoard_C|GetAddTeamsToThisBox (Variables|Default|GetTeam1Stats)) _returnvalue_4))
      (bind _asbp_game_state_2 (Utilities|Casting|CastToBP_GameState (Game|GetGameState)))
      (for _array_element_2 (Variables|/Script/FPSProject.FPSGameState|GetTeam2PlayerControllers _asbp_game_state_2)
        (bind _returnvalue_5 (UserInterface|CreateWidget "/Game/UI/PlayerStats.PlayerStats_C"))
        (Class|VerticalBox|AddChildtoVerticalBox (Variables|/Game/UI/TeamScoreBoard.TeamScoreBoard_C|GetAddTeamsToThisBox (Variables|Default|GetTeam2Stats)) _returnvalue_5))
      (UserInterface|Viewport|AddtoViewport (Variables|Default|GetScoreBoardUI) 5))))

(event EventTriggerAddAliveUIBlueprint
  ;[1 1 1] GameUI
  (CallFunction|AddGameUItoClient))

(event EventUpdateScoreBoardUIBlueprint
  (CallFunction|UpdatePlayerStats))

(event EventUpdateScoreUIBlueprint
  ;[1 1 1] ScoreUI
  (CallFunction|UpdateScore))

(event EventAddScoreBoardUIBlueprint
  ;[1 1 1] base scoreboard
  (CallFunction|AddScoreBoardtoClient))

(fn ConstructionScript)